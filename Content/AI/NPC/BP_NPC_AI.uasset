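; BP_NPC_AI is the AI controller that drives BP_NPC characters and sets up their patrol behavior.
; On BeginPlay it runs the BT_NPC behavior tree, then casts and caches the controlled BP_NPC pawn.
; It seeds the blackboard with the loop flag and wait time from the pawn's PatrolPath, plus an initial forward direction.
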(event EventBeginPlay
  (bind _returnvalue (AI|GetBlackboard 0))
  (AI|RunBehaviorTree "/Game/AI/NPC/BT_NPC.BT_NPC")
  (bind _asbp_npc (Utilities|Casting|CastToBP_NPC (Pawn|GetControlledPawn)))
  (Variables|Default|SetControlledPawn _asbp_npc)
  (AI|Components|Blackboard|SetValueasBool _returnvalue (Utilities|Name|MakeLiteralName "bLoopPath") (Variables|/Game/AI/NPC/BP_PatrolPath.BP_PatrolPath_C|GetbLoopPath (Variables|/Game/AI/NPC/BP_NPC.BP_NPC_C|GetPatrolPath _asbp_npc)))
  (Class|BlackboardComponent|SetValueasInt _returnvalue (Utilities|Name|MakeLiteralName "Direction") 1)
  (AI|Components|Blackboard|SetValueasFloat _returnvalue (Utilities|Name|MakeLiteralName "PatrolPointWaitTime") (Variables|/Game/AI/NPC/BP_PatrolPath.BP_PatrolPath_C|GetPatrolPointWaitTime (Variables|/Game/AI/NPC/BP_NPC.BP_NPC_C|GetPatrolPath _asbp_npc))))

(event EventTick
  (params (DeltaSeconds :type Float%20%28single-precision%29)))

(fn ConstructionScript)